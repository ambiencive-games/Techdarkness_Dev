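; Base world actor for a pickup that can be collected into the grid-style inventory.
; On BeginPlay it constructs a default item object if none is set, holding grid dimensions, normal and rotated icons, and its own class.
; Interact passes that object to the caller's inventory component and, if the add succeeds, calls a server-named event that destroys the actor.
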(event `self.ReceiveBeginPlay`
  (if (not (`KismetSystemLibrary.IsValid` (`self.Item_Object`)))
    (bind _item_object (`self.Get_Defoult_Item_Object`))
    (set `self.Item_Object` _item_object)))

(event `/Game/Game/BP/Main/Inventory/Blueprint/Inventory/BPI_Interact.Interact`
  (params (Inventory_Component :type "/Game/Game/BP/Main/Inventory/Blueprint/Inventory/BPC_Inventory Object Reference"))
  (bind _added (`/Game/Game/BP/Main/Inventory/Blueprint/Inventory/BPC_Inventory.Try_Add_Item` Inventory_Component (`self.Item_Object`)))
  (if _added
    (`self.Server_Destroy_Item`)))

(event `Server_Destroy_Item`
  (`self.K2_DestroyActor`))

(fn `Get_Defoult_Item_Object`
  (returns (Item_Object :type "/Game/Game/BP/Main/Inventory/Blueprint/Inventory/BP_Base_Item_Object Object Reference"))
  (bind _returnvalue (`|GenericCreateObject` self "/Game/Game/BP/Main/Inventory/Blueprint/Inventory/BP_Base_Item_Object.BP_Base_Item_Object_C" (make `IntPoint` 2 1) "/Engine/EngineResources/AICON-Green.AICON-Green" (`GameplayStatics.GetObjectClass` self) "/Engine/EngineResources/AICON-Red.AICON-Red"))
  (return _returnvalue))

(fn `UserConstructionScript`)